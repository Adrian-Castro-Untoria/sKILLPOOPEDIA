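; BP_EndOfGameTrigger is a volume actor that ends the game when the player character enters it.
; On BeginPlay it caches the third-person character and pre-creates the WP_EndScreen widget.
; When a BP_ThirdPersonCharacter overlaps the box, it shows that widget, pauses the game, reveals the mouse cursor and switches input to Game and UI focused on the end screen.
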(event OnComponentBeginOverlap(Box)
  (params (OverlappedComponent :type Primitive%20Component%20Object%20Reference) (OtherActor :type Actor%20Object%20Reference) (OtherComp :type Primitive%20Component%20Object%20Reference) (OtherBodyIndex :type Integer) (bFromSweep :type Boolean) (SweepResult :type Hit%20Result%20Structure%20%28by%20ref%29))
  (bind _returnvalue (Game|GetPlayerController 0))
  (Utilities|Casting|CastToBP_ThirdPersonCharacter OtherActor)
  (UserInterface|Viewport|AddtoViewport (Variables|Ref|GetEndScreenWidget_Ref) 0)
  (Game|SetGamePaused true)
  (Variables|/Script/Engine.PlayerController|SetbShowMouseCursor _returnvalue true)
  (Input|SetInputModeGameandUI _returnvalue (Variables|Ref|GetEndScreenWidget_Ref) "DoNotLock" false false))

(event EventBeginPlay
  (bind _asbp_third_person_character (Utilities|Casting|CastToBP_ThirdPersonCharacter (Game|GetPlayerCharacter 0)))
  (Variables|Ref|SetCharacter_Ref _asbp_third_person_character)
  (bind _returnvalue (UserInterface|CreateWidget "/Game/UI/Widget/WP_EndScreen.WP_EndScreen_C"))
  (Variables|Ref|SetEndScreenWidget_Ref _returnvalue))

(fn ConstructionScript)