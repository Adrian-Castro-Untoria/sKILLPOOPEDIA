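; BP_GoodPortail is a one-use portal that teleports the third-person player character to a set Teleport location.
; At BeginPlay it applies a material to its two portal meshes.
; If the SpiderGameInstance Portals flag is set, it unhides both meshes and enables the Detection collision.
; Overlapping Detection moves the character to Teleport and then destroys the portal.
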(event OnComponentBeginOverlap(detection)
  (params (OverlappedComponent :type Primitive%20Component%20Object%20Reference) (OtherActor :type Actor%20Object%20Reference) (OtherComp :type Primitive%20Component%20Object%20Reference) (OtherBodyIndex :type Integer) (bFromSweep :type Boolean) (SweepResult :type Hit%20Result%20Structure%20%28by%20ref%29))
  (bind _asbp_third_person_character (Utilities|Casting|CastToBP_ThirdPersonCharacter OtherActor))
  (Transformation|SetActorLocation _asbp_third_person_character (Variables|Default|Getteleport) false false)
  (Actor|DestroyActor))

(event EventBeginPlay
  (Rendering|Material|SetMaterial (Variables|Default|GetPortail) 0 (Variables|Default|GetMaterial))
  (Utilities|Casting|CastToBP_ThirdPersonCharacter (Game|GetPlayerCharacter 0))
  (bind _asspider_game_instance (Utilities|Casting|CastToSpiderGameInstance (Game|GetGameInstance)))
  (if (Variables|/Game/ThirdPerson/Blueprints/SpiderGameInstance.SpiderGameInstance_C|GetPortals _asspider_game_instance)
    (Development|SetHiddeninGame (Variables|Default|GetPortail1) false false)
    (Collision|SetCollisionEnabled (Variables|Default|Getdetection) "QueryAndPhysics")))

(fn ConstructionScript)