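; BP_GravityCrystal is an environment crystal that changes the player character's gravity while they are within its range.
; On BeginPlay it caches the character's default gravity scale, and reveals and enables collision on the mesh and range only if the game instance's GravityCrystals flag is set.
; Overlapping CrystalRange applies NewGravity, and leaving restores the cached default.
; The construction script sizes the range uniformly from RangeScale.
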(event OnComponentBeginOverlap(CrystalRange)
  (params (OverlappedComponent :type Primitive%20Component%20Object%20Reference) (OtherActor :type Actor%20Object%20Reference) (OtherComp :type Primitive%20Component%20Object%20Reference) (OtherBodyIndex :type Integer) (bFromSweep :type Boolean) (SweepResult :type Hit%20Result%20Structure%20%28by%20ref%29))
  (Utilities|Casting|CastToBP_ThirdPersonCharacter OtherActor)
  (Variables|/Script/Engine.CharacterMovementComponent|SetGravityScale (Variables|/Script/Engine.Character|GetCharacterMovement (Variables|Ref|GetCharacter_Ref)) (Variables|Default|GetNewGravity)))

(event OnComponentEndOverlap(CrystalRange)
  (params (OverlappedComponent :type Primitive%20Component%20Object%20Reference) (OtherActor :type Actor%20Object%20Reference) (OtherComp :type Primitive%20Component%20Object%20Reference) (OtherBodyIndex :type Integer))
  (Utilities|Casting|CastToBP_ThirdPersonCharacter OtherActor)
  (Variables|/Script/Engine.CharacterMovementComponent|SetGravityScale (Variables|/Script/Engine.Character|GetCharacterMovement (Variables|Ref|GetCharacter_Ref)) (Variables|Default|GetDefaultGravity)))

(event EventBeginPlay
  (bind _crystalrange (Variables|Default|GetCrystalRange))
  (bind _asspider_game_instance (Utilities|Casting|CastToSpiderGameInstance (Game|GetGameInstance)))
  (Variables|Ref|SetGameInstance_Ref _asspider_game_instance)
  (bind _asbp_third_person_character (Utilities|Casting|CastToBP_ThirdPersonCharacter (Game|GetPlayerCharacter 0)))
  (Variables|Ref|SetCharacter_Ref _asbp_third_person_character)
  (Variables|Default|SetDefaultGravity (Variables|/Script/Engine.CharacterMovementComponent|GetGravityScale (Variables|/Script/Engine.Character|GetCharacterMovement (Variables|Ref|GetCharacter_Ref))))
  (if (Variables|/Game/ThirdPerson/Blueprints/SpiderGameInstance.SpiderGameInstance_C|GetGravity%20Crystals (Variables|Ref|GetGameInstance_Ref))
    (Development|SetHiddeninGame _crystalrange false false)
    (Collision|SetCollisionEnabled _crystalrange "QueryAndPhysics")))

(fn ConstructionScript
  (bind _rangescale (Variables|Default|GetRangeScale))
  (Transformation|SetRelativeScale3D (Variables|Default|GetCrystalRange) (Math|Vector|MakeVector _rangescale _rangescale _rangescale)))