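; Falling, moving platform, going by its name, driven by an InterpToMovement component.
; The construction script sets the movement duration from Duration1 and adds Pos as a relative control point.
; When a BP_ThirdPersonCharacter begins overlapping the Box, it prints a debug "Hello" and appends MoveToPos1 as another relative control point.
; Each overlap appends again, with no guard and no FinaliseControlPoints call.
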(event OnComponentBeginOverlap(Box)
  (params (OverlappedComponent :type Primitive%20Component%20Object%20Reference) (OtherActor :type Actor%20Object%20Reference) (OtherComp :type Primitive%20Component%20Object%20Reference) (OtherBodyIndex :type Integer) (bFromSweep :type Boolean) (SweepResult :type Hit%20Result%20Structure%20%28by%20ref%29))
  (Utilities|Casting|CastToBP_ThirdPersonCharacter OtherActor)
  (Development|PrintString "Hello")
  (Class|InterptoMovementComponent|AddControlPointPosition (Variables|Default|GetInterpToMovement) (Variables|Default|GetMoveToPos1) true))

(fn ConstructionScript
  (Variables|/Script/Engine.InterpToMovementComponent|SetDuration (Variables|Default|GetInterpToMovement) (Variables|Default|GetDuration1))
  (Class|InterptoMovementComponent|AddControlPointPosition (Variables|Default|GetInterpToMovement) (Variables|Default|GetPos) true))