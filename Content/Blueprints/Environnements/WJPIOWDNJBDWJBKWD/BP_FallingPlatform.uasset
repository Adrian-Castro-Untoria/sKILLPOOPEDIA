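; Platform actor that falls when the player character steps on it and rises back some time after they leave.
; BeginPlay stores the start position, derives the target from FallDistance and uses FallTime as the timeline's play rate.
; Box overlap plays the FallingTime timeline through a DoOnce, lerping between both positions, with a delayed reset chained to its update.
; End overlap reverses the timeline from its end after a fixed delay.
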(event OnComponentBeginOverlap(Box)
  (params (OverlappedComponent :type Primitive%20Component%20Object%20Reference) (OtherActor :type Actor%20Object%20Reference) (OtherComp :type Primitive%20Component%20Object%20Reference) (OtherBodyIndex :type Integer) (bFromSweep :type Boolean) (SweepResult :type Hit%20Result%20Structure%20%28by%20ref%29))
  (Utilities|Casting|CastToBP_ThirdPersonCharacter OtherActor)
  (Development|PrintString "Hello")
  (Variables|Default|SetPlayerDessus? true)
  (Utilities|FlowControl|DoOnce false :!label _label
    (:Completed
      (bind _newtrack_0 (Timeline|FallingTime PlayFromStart)
        (:Update
          (Transformation|SetActorLocation (Math|Vector|Lerp(Vector) (Variables|Default|GetInitialPosition) (Variables|Default|GetTargetPosition) _newtrack_0) false false)
          (Utilities|FlowControl|Delay 1e+01)
          (goto _label Reset))))))

(event OnComponentEndOverlap(Box)
  (params (OverlappedComponent :type Primitive%20Component%20Object%20Reference) (OtherActor :type Actor%20Object%20Reference) (OtherComp :type Primitive%20Component%20Object%20Reference) (OtherBodyIndex :type Integer))
  (Utilities|Casting|CastToBP_ThirdPersonCharacter OtherActor)
  (Utilities|FlowControl|Delay 1e+01)
  (bind _newtrack_0 (Timeline|FallingTime ReverseFromEnd)
    (:Update
      (Transformation|SetActorLocation (Math|Vector|Lerp(Vector) (Variables|Default|GetInitialPosition) (Variables|Default|GetTargetPosition) _newtrack_0) false false)
      (Utilities|FlowControl|Delay 1e+01)
      (Utilities|FlowControl|DoOnce false) ; enters at Reset
    )))

(event EventBeginPlay
  (Variables|Default|SetInitialPosition (Transformation|GetActorLocation))
  (Variables|Default|SetTargetPosition (- (Variables|Default|GetInitialPosition) (Variables|Default|GetFallDistance)))
  (Components|Timeline|SetPlayRate (Variables|Default|GetFallingTime) (Variables|Default|GetFallTime)))

(fn ConstructionScript)