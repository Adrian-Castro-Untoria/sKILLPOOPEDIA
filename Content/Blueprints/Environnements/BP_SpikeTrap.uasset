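; BP_SpikeTrap is an environment spike trap with a Trap mesh and a SpikesActivate event that plays its hide animation once.
; BeginPlay leads only to an empty sequence, so the trap does nothing on its own.
; Disconnected leftover logic would cache the player character and game instance, show the trap with collision, loop SpikesActivate on a timer, and reposition the Box component.
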(event Custom|SpikesActivate
  (Components|Animation|PlayAnimation (Variables|Default|GetTrap) "/Game/LevelPrototyping/source/SpikeTrap_HideAnimation_Anim.SpikeTrap_HideAnimation_Anim" false))

(event EventBeginPlay
  (Utilities|FlowControl|Sequence))

(fn ConstructionScript)