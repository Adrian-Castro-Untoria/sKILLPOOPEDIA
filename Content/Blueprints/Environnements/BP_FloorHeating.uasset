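; BP_FloorHeating is a heated floor hazard that damages the third-person character standing in its box trigger.
; Entering the box starts a delayed StartDamage timer, which begins a looping timer applying DamagePerSecond every second if the player is still inside.
; Leaving clears only the delayed timer, so damage that has already started keeps looping.
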(event OnComponentBeginOverlap(Box)
  (params (OverlappedComponent :type Primitive%20Component%20Object%20Reference) (OtherActor :type Actor%20Object%20Reference) (OtherComp :type Primitive%20Component%20Object%20Reference) (OtherBodyIndex :type Integer) (bFromSweep :type Boolean) (SweepResult :type Hit%20Result%20Structure%20%28by%20ref%29))
  (bind _asbp_third_person_character (Utilities|Casting|CastToBP_ThirdPersonCharacter OtherActor))
  (Variables|Default|SetBlsPlayerOnFloor true)
  (Utilities|Time|SetTimerbyFunctionName 0 "StartDamage" 5.0)
  (Development|PrintString "Hello"))

(event OnComponentEndOverlap(Box)
  (params (OverlappedComponent :type Primitive%20Component%20Object%20Reference) (OtherActor :type Actor%20Object%20Reference) (OtherComp :type Primitive%20Component%20Object%20Reference) (OtherBodyIndex :type Integer))
  (Utilities|Casting|CastToBP_ThirdPersonCharacter OtherActor)
  (Variables|Default|SetBlsPlayerOnFloor false)
  (Utilities|Time|ClearTimerbyFunctionName 0 "StartDamage"))

(event Custom|StartDamage
  (if (Variables|Default|GetBlsPlayerOnFloor)
    (Development|PrintString "HELLOOO")
    (Utilities|Time|SetTimerbyEvent (delegate Custom|CustomEvent) 1.0 true)))

(event Custom|CustomEvent
  (Game|Damage|ApplyDamage (stale OnComponentBeginOverlap(Box) _asbp_third_person_character) (Variables|Default|GetDamagePerSecond) 0 0))

(fn ConstructionScript)