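; BP_SpeedBoost is a single-use pickup that temporarily boosts the speed of the BP_ThirdPersonCharacter that touches it.
; Overlapping its collision sphere raises the character's max walk and fly speeds, prints a debug string, hides the visible sphere and disables collision.
; After a five-second delay it sets both speeds to hardcoded lower values rather than saved originals; the pickup stays hidden and is never destroyed.
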(event OnComponentBeginOverlap(Sphere1)
  (params (OverlappedComponent :type Primitive%20Component%20Object%20Reference) (OtherActor :type Actor%20Object%20Reference) (OtherComp :type Primitive%20Component%20Object%20Reference) (OtherBodyIndex :type Integer) (bFromSweep :type Boolean) (SweepResult :type Hit%20Result%20Structure%20%28by%20ref%29))
  (bind _asbp_third_person_character (Utilities|Casting|CastToBP_ThirdPersonCharacter OtherActor))
  (Variables|/Script/Engine.CharacterMovementComponent|SetMaxWalkSpeed (Variables|/Script/Engine.Character|GetCharacterMovement _asbp_third_person_character) 2.4e+03)
  (Variables|/Script/Engine.CharacterMovementComponent|SetMaxFlySpeed (Variables|/Script/Engine.Character|GetCharacterMovement _asbp_third_person_character) 1.8e+03)
  (Development|PrintString "Hello")
  (Rendering|SetVisibility (Variables|Default|GetSphere) false false)
  (Collision|SetCollisionEnabled (Variables|Default|GetSphere1) "NoCollision")
  (Utilities|FlowControl|Delay 5.0)
  (Variables|/Script/Engine.CharacterMovementComponent|SetMaxWalkSpeed (Variables|/Script/Engine.Character|GetCharacterMovement _asbp_third_person_character) 1.2e+03)
  (Variables|/Script/Engine.CharacterMovementComponent|SetMaxFlySpeed (Variables|/Script/Engine.Character|GetCharacterMovement _asbp_third_person_character) 9e+02))

(fn ConstructionScript)