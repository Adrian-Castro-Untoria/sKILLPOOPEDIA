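; Spike trap actor that damages the third-person player character.
; On BeginPlay it reveals the skeletal mesh and enables its collision only if the game instance's SpikySituation flag is set.
; Box overlap prints a debug string and deals one damage to the character, without checking that flag.
; Tick applies DamageValue while InDanger is true, but nothing here sets InDanger, and the mesh overlap events are empty.
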(event OnComponentBeginOverlap(SkeletalMesh)
  (params (OverlappedComponent :type Primitive%20Component%20Object%20Reference) (OtherActor :type Actor%20Object%20Reference) (OtherComp :type Primitive%20Component%20Object%20Reference) (OtherBodyIndex :type Integer) (bFromSweep :type Boolean) (SweepResult :type Hit%20Result%20Structure%20%28by%20ref%29)))

(event OnComponentEndOverlap(SkeletalMesh)
  (params (OverlappedComponent :type Primitive%20Component%20Object%20Reference) (OtherActor :type Actor%20Object%20Reference) (OtherComp :type Primitive%20Component%20Object%20Reference) (OtherBodyIndex :type Integer)))

(event OnComponentBeginOverlap(Box)
  (params (OverlappedComponent :type Primitive%20Component%20Object%20Reference) (OtherActor :type Actor%20Object%20Reference) (OtherComp :type Primitive%20Component%20Object%20Reference) (OtherBodyIndex :type Integer) (bFromSweep :type Boolean) (SweepResult :type Hit%20Result%20Structure%20%28by%20ref%29))
  (Development|PrintString "WHY")
  (bind _asbp_third_person_character (Utilities|Casting|CastToBP_ThirdPersonCharacter OtherActor))
  (Default|TakingDamage _asbp_third_person_character 1))

(event EventBeginPlay
  (bind _skeletalmesh (Variables|Default|GetSkeletalMesh))
  (bind _asbp_third_person_character (Utilities|Casting|CastToBP_ThirdPersonCharacter (Game|GetPlayerCharacter 0)))
  (Variables|Ref|SetCharacter_Ref _asbp_third_person_character)
  (bind _asspider_game_instance (Utilities|Casting|CastToSpiderGameInstance (Game|GetGameInstance)))
  (bind _output_get (Variables|Ref|SetGameInstance_Ref _asspider_game_instance))
  (if (Variables|/Game/ThirdPerson/Blueprints/SpiderGameInstance.SpiderGameInstance_C|GetSpikySituation _output_get)
    (Development|SetHiddeninGame _skeletalmesh false false)
    (Collision|SetCollisionEnabled _skeletalmesh "QueryAndPhysics")))

(event EventTick
  (params (DeltaSeconds :type Float%20%28single-precision%29))
  (if (Variables|Default|GetInDanger)
    (Default|TakingDamage (Variables|Ref|GetCharacter_Ref) (Variables|Default|GetDamageValue))))

(fn ConstructionScript)