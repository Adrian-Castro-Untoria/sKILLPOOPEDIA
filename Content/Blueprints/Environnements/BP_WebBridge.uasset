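; BP_WebBridge is an environment bridge that appears and becomes solid only when the game instance's WebBridges flag is set.
; On BeginPlay it caches the third-person character and SpiderGameInstance, then reads that flag.
; When true it unhides the Bridge component and enables query and physics collision, otherwise it only disables collision.
; The state is evaluated once at BeginPlay, and the cached character is not otherwise used here.
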(event EventBeginPlay
  (bind _bridge (Variables|Default|GetBridge))
  (bind _asbp_third_person_character (Utilities|Casting|CastToBP_ThirdPersonCharacter (Game|GetPlayerCharacter 0)))
  (Variables|Default|SetAs%20BP%20Third%20Person%20Character _asbp_third_person_character)
  (bind _asspider_game_instance (Utilities|Casting|CastToSpiderGameInstance (Game|GetGameInstance)))
  (bind _output_get (Variables|Default|SetAs%20Spider%20Game%20Instance _asspider_game_instance))
  (if (Variables|/Game/ThirdPerson/Blueprints/SpiderGameInstance.SpiderGameInstance_C|GetWebBridges _output_get)
    (Development|SetHiddeninGame _bridge false false)
    (Collision|SetCollisionEnabled _bridge "QueryAndPhysics")
    (else
      (Collision|SetCollisionEnabled (Variables|Default|GetBridge) "NoCollision"))))

(fn ConstructionScript)