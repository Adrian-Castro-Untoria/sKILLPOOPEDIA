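; BP_MoreJumpads is an optional jump pad that activates when the SpiderGameInstance's BetterTrampolines flag is set.
; On BeginPlay, that flag unhides the Cube, enables collision on the Box trigger and prints a debug string.
; Box overlap launches BP_ThirdPersonCharacter by HauteurSaut, overriding its velocity, and sets PlayerDessus.
; Any end overlap clears PlayerDessus, which nothing in this graph reads.
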(event OnComponentBeginOverlap(Box)
  (params (OverlappedComponent :type Primitive%20Component%20Object%20Reference) (OtherActor :type Actor%20Object%20Reference) (OtherComp :type Primitive%20Component%20Object%20Reference) (OtherBodyIndex :type Integer) (bFromSweep :type Boolean) (SweepResult :type Hit%20Result%20Structure%20%28by%20ref%29))
  (bind _asbp_third_person_character (Utilities|Casting|CastToBP_ThirdPersonCharacter OtherActor))
  (Variables|Default|SetPlayerDessus? true)
  (Character|LaunchCharacter _asbp_third_person_character (Variables|Default|GetHauteurSaut) true true))

(event OnComponentEndOverlap(Box)
  (params (OverlappedComponent :type Primitive%20Component%20Object%20Reference) (OtherActor :type Actor%20Object%20Reference) (OtherComp :type Primitive%20Component%20Object%20Reference) (OtherBodyIndex :type Integer))
  (Variables|Default|SetPlayerDessus? false))

(event EventBeginPlay
  (bind _asspider_game_instance (Utilities|Casting|CastToSpiderGameInstance (Game|GetGameInstance)))
  (bind _output_get (Variables|Default|SetGameInstance_Ref _asspider_game_instance))
  (if (Variables|/Game/ThirdPerson/Blueprints/SpiderGameInstance.SpiderGameInstance_C|GetBetterTrampolines _output_get)
    (Development|SetHiddeninGame (Variables|Default|GetCube) false true)
    (Collision|SetCollisionEnabled (Variables|Default|GetBox) "QueryAndPhysics")
    (Development|PrintString "Popo ?")))

(fn ConstructionScript)