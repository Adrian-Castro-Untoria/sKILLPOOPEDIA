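; BP_OpposingWinds is a wind zone that pushes the third-person player along its arrow's forward direction, enabled on BeginPlay only when SpiderGameInstance's OpposingWinds flag is set.
; WindArea overlaps track whether the player is inside.
; Tick ramps the force up to a maximum while inside and decays it outside, so the push lingers after exit.
; Force is applied through additive per-frame LaunchCharacter calls scaled by delta time.
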(event OnComponentBeginOverlap(WindArea)
  (params (OverlappedComponent :type Primitive%20Component%20Object%20Reference) (OtherActor :type Actor%20Object%20Reference) (OtherComp :type Primitive%20Component%20Object%20Reference) (OtherBodyIndex :type Integer) (bFromSweep :type Boolean) (SweepResult :type Hit%20Result%20Structure%20%28by%20ref%29))
  (Utilities|Casting|CastToBP_ThirdPersonCharacter OtherActor)
  (Variables|Default|SetbPlayerInside true))

(event OnComponentEndOverlap(WindArea)
  (params (OverlappedComponent :type Primitive%20Component%20Object%20Reference) (OtherActor :type Actor%20Object%20Reference) (OtherComp :type Primitive%20Component%20Object%20Reference) (OtherBodyIndex :type Integer))
  (Utilities|Casting|CastToBP_ThirdPersonCharacter OtherActor)
  (Variables|Default|SetbPlayerInside false))

(event EventBeginPlay
  (bind _windarea (Variables|Default|GetWindArea))
  (bind _asbp_third_person_character (Utilities|Casting|CastToBP_ThirdPersonCharacter (Game|GetPlayerCharacter 0)))
  (Variables|Default|SetAs%20BP%20Third%20Person%20Character _asbp_third_person_character)
  (bind _asspider_game_instance (Utilities|Casting|CastToSpiderGameInstance (Game|GetGameInstance)))
  (if (Variables|/Game/ThirdPerson/Blueprints/SpiderGameInstance.SpiderGameInstance_C|GetOpposing%20Winds _asspider_game_instance)
    (Development|SetHiddeninGame _windarea false false)
    (Collision|SetCollisionEnabled _windarea "QueryAndPhysics")))

(event EventTick
  (params (DeltaSeconds :type Float%20%28single-precision%29))
  (Variables|Default|SetDelta%20Seconds DeltaSeconds)
  (Utilities|FlowControl|Sequence
    (:then_0
      (Variables|Default|SetWindDirection (Math|Vector|GetForwardVector (Variables|Default|GetArrow)))
      (if (Variables|Default|GetbPlayerInside)
        (Variables|Default|SetCurrentFoce (Math|Float|Clamp(Float) (+ (* (Variables|Default|GetDelta%20Seconds) (Variables|Default|GetBuildUpSpeed)) (Variables|Default|GetCurrentFoce)) 0.0 (Variables|Default|GetMaxForce)))
        (else
          (Variables|Default|SetCurrentFoce (Math|Float|Clamp(Float) (- (Variables|Default|GetCurrentFoce) (* (Variables|Default|GetDelta%20Seconds) (Variables|Default|GetDecaySpeed))) 0.0 (Variables|Default|GetMaxForce))))))
    (:then_1
      (if (> (Variables|Default|GetCurrentFoce) 0.0)
        (Character|LaunchCharacter (Variables|Default|GetAs%20BP%20Third%20Person%20Character) (* (* (Variables|Default|GetCurrentFoce) (Variables|Default|GetDelta%20Seconds)) (Variables|Default|GetWindDirection)) false false)))))

(fn ConstructionScript)