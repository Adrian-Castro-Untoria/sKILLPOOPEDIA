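; Sugar cube pickup that gives the player character a temporary speed boost.
; On BeginPlay it caches the character and its default walk speed, then shows the cube and enables collision if the SugarCubes flag in SpiderGameInstance is set.
; Player overlap applies the boost speed and hides the cube, then restores the cached speed after a delay and destroys the actor.
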(event OnComponentBeginOverlap(Collision)
  (params (OverlappedComponent :type Primitive%20Component%20Object%20Reference) (OtherActor :type Actor%20Object%20Reference) (OtherComp :type Primitive%20Component%20Object%20Reference) (OtherBodyIndex :type Integer) (bFromSweep :type Boolean) (SweepResult :type Hit%20Result%20Structure%20%28by%20ref%29))
  (Utilities|Casting|CastToBP_ThirdPersonCharacter OtherActor)
  (Variables|/Script/Engine.CharacterMovementComponent|SetMaxWalkSpeed (Variables|/Script/Engine.Character|GetCharacterMovement (Variables|Default|GetCharacter_Ref)) (Variables|Default|GetBoostSpeed))
  (Development|SetHiddeninGame (Variables|Default|GetCube) true true)
  (Collision|SetCollisionEnabled (Variables|Default|GetCollision) "NoCollision")
  (Utilities|FlowControl|Delay (Variables|Default|GetBoostDuration))
  (Variables|/Script/Engine.CharacterMovementComponent|SetMaxWalkSpeed (Variables|/Script/Engine.Character|GetCharacterMovement (Variables|Default|GetCharacter_Ref)) (Variables|Default|GetDefaultWalkSpeed))
  (Actor|DestroyActor))

(event EventBeginPlay
  (bind _asbp_third_person_character (Utilities|Casting|CastToBP_ThirdPersonCharacter (Game|GetPlayerCharacter 0)))
  (Variables|Default|SetCharacter_Ref _asbp_third_person_character)
  (bind _asspider_game_instance (Utilities|Casting|CastToSpiderGameInstance (Game|GetGameInstance)))
  (Variables|Default|SetGameInstance_Ref _asspider_game_instance)
  (Variables|Default|SetDefaultWalkSpeed (Variables|/Script/Engine.CharacterMovementComponent|GetMaxWalkSpeed (Variables|/Script/Engine.Character|GetCharacterMovement (Variables|Default|GetCharacter_Ref))))
  (if (Variables|/Game/ThirdPerson/Blueprints/SpiderGameInstance.SpiderGameInstance_C|GetSugarCubes (Variables|Default|GetGameInstance_Ref))
    (Development|SetHiddeninGame (Variables|Default|GetCube) false true)
    (Collision|SetCollisionEnabled (Variables|Default|GetCollision) "QueryAndPhysics")))

(fn ConstructionScript)