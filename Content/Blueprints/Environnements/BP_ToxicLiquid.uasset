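; Toxic liquid hazard that damages the player while a character overlaps its cylinder.
; On BeginPlay it caches the player character and SpiderGameInstance, then shows the cylinder and enables its collision if the ToxicLiquid flag is set.
; Any Character overlap toggles InDanger, and Tick then calls TakingDamage on the cached player every frame, with no delta-time scaling.
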(event OnComponentBeginOverlap(Cylinder)
  (params (OverlappedComponent :type Primitive%20Component%20Object%20Reference) (OtherActor :type Actor%20Object%20Reference) (OtherComp :type Primitive%20Component%20Object%20Reference) (OtherBodyIndex :type Integer) (bFromSweep :type Boolean) (SweepResult :type Hit%20Result%20Structure%20%28by%20ref%29))
  (Class|KismetSystemLibrary|IsObjectOfSoftClass OtherActor "/Script/Engine.Character"
    (:True
      (Variables|Default|SetInDanger true))))

(event OnComponentEndOverlap(Cylinder)
  (params (OverlappedComponent :type Primitive%20Component%20Object%20Reference) (OtherActor :type Actor%20Object%20Reference) (OtherComp :type Primitive%20Component%20Object%20Reference) (OtherBodyIndex :type Integer))
  (Class|KismetSystemLibrary|IsObjectOfSoftClass OtherActor "/Script/Engine.Character"
    (:True
      (Variables|Default|SetInDanger false))))

(event EventBeginPlay
  (bind _cylinder (Variables|Default|GetCylinder))
  (bind _asbp_third_person_character (Utilities|Casting|CastToBP_ThirdPersonCharacter (Game|GetPlayerCharacter 0)))
  (Variables|Ref|SetCharacter_Ref _asbp_third_person_character)
  (bind _asspider_game_instance (Utilities|Casting|CastToSpiderGameInstance (Game|GetGameInstance)))
  (bind _output_get (Variables|Ref|SetGameInstance_Ref _asspider_game_instance))
  (if (Variables|/Game/ThirdPerson/Blueprints/SpiderGameInstance.SpiderGameInstance_C|GetToxicLiquid _output_get)
    (Development|SetHiddeninGame _cylinder false false)
    (Collision|SetCollisionEnabled _cylinder "QueryAndPhysics")))

(event EventTick
  (params (DeltaSeconds :type Float%20%28single-precision%29))
  (if (Variables|Default|GetInDanger)
    (Default|TakingDamage (Variables|Ref|GetCharacter_Ref) (Variables|Default|GetDamageValue))))

(fn ConstructionScript)