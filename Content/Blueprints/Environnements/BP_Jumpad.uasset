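; BP_Jumpad is a jump pad that launches the third-person player character when it enters the pad's Box trigger.
; The launch overrides the character's velocity with HauteurSaut, and PlayerDessus is set while overlapping and cleared on end overlap.
; On BeginPlay, pads of the More Trampoline type show their cube and enable collision only if the Trampolines flag in SpiderGameInstance is set.
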(event OnComponentBeginOverlap(Box)
  (params (OverlappedComponent :type Primitive%20Component%20Object%20Reference) (OtherActor :type Actor%20Object%20Reference) (OtherComp :type Primitive%20Component%20Object%20Reference) (OtherBodyIndex :type Integer) (bFromSweep :type Boolean) (SweepResult :type Hit%20Result%20Structure%20%28by%20ref%29))
  (bind _asbp_third_person_character (Utilities|Casting|CastToBP_ThirdPersonCharacter OtherActor))
  (Variables|Default|SetPlayerDessus? true)
  (Character|LaunchCharacter _asbp_third_person_character (Variables|Default|GetHauteurSaut) true true))

(event OnComponentEndOverlap(Box)
  (params (OverlappedComponent :type Primitive%20Component%20Object%20Reference) (OtherActor :type Actor%20Object%20Reference) (OtherComp :type Primitive%20Component%20Object%20Reference) (OtherBodyIndex :type Integer))
  (Variables|Default|SetPlayerDessus? false))

(event EventBeginPlay
  (bind _asspider_game_instance (Utilities|Casting|CastToSpiderGameInstance (Game|GetGameInstance)))
  (Variables|Ref|SetGameInstance_Ref _asspider_game_instance)
  (switch Utilities|FlowControl|Switch|SwitchonEJumpPadType (Variables|Default|GetEJumpPadType)
    (:NewEnumerator1
      (if (Variables|/Game/ThirdPerson/Blueprints/SpiderGameInstance.SpiderGameInstance_C|GetTrampolines (Variables|Ref|GetGameInstance_Ref))
        (Development|SetHiddeninGame (Variables|Default|GetCube) false true)
        (Collision|SetCollisionEnabled (Variables|Default|GetBox) "QueryAndPhysics")
        (else
          (Development|SetHiddeninGame (Variables|Default|GetCube) true true)
          (Collision|SetCollisionEnabled (Variables|Default|GetBox) "NoCollision"))))))

(fn ConstructionScript)