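; Fly pickup actor that restores health to the player's spider, active only when the TastyFlies flag is set in SpiderGameInstance.
; On BeginPlay it reveals its sphere and enables collision if that flag is true.
; When BP_ThirdPersonCharacter overlaps it below max health, it increments Health in the GameInstance, refreshes the character's health widget and destroys itself.
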(event OnComponentBeginOverlap(Collision)
  (params (OverlappedComponent :type Primitive%20Component%20Object%20Reference) (OtherActor :type Actor%20Object%20Reference) (OtherComp :type Primitive%20Component%20Object%20Reference) (OtherBodyIndex :type Integer) (bFromSweep :type Boolean) (SweepResult :type Hit%20Result%20Structure%20%28by%20ref%29))
  (bind _gameinstance_ref (Variables|Default|GetGameInstance_Ref))
  (bind _gameinstance_ref_2 (Variables|Default|GetGameInstance_Ref))
  (bind _asbp_third_person_character (Utilities|Casting|CastToBP_ThirdPersonCharacter OtherActor))
  (Variables|Default|SetCharacter_Ref _asbp_third_person_character)
  (if (< (Variables|/Game/ThirdPerson/Blueprints/SpiderGameInstance.SpiderGameInstance_C|GetHealth _gameinstance_ref_2) (Variables|/Game/ThirdPerson/Blueprints/SpiderGameInstance.SpiderGameInstance_C|GetMaxHealth _gameinstance_ref_2))
    (bind _result (Math|Integer|IncrementInt (Variables|/Game/ThirdPerson/Blueprints/SpiderGameInstance.SpiderGameInstance_C|GetHealth _gameinstance_ref))
      (:%20%20
        (Variables|/Game/ThirdPerson/Blueprints/SpiderGameInstance.SpiderGameInstance_C|SetHealth _gameinstance_ref _result)
        (Default|UpdateHP (Variables|/Game/Characters/areigne/BP_ThirdPersonCharacter.BP_ThirdPersonCharacter_C|GetHealthWidget_Ref (Variables|Default|GetCharacter_Ref)))
        (Actor|DestroyActor)))))

(event EventBeginPlay
  (bind _asspider_game_instance (Utilities|Casting|CastToSpiderGameInstance (Game|GetGameInstance)))
  (bind _output_get (Variables|Default|SetGameInstance_Ref _asspider_game_instance))
  (if (Variables|/Game/ThirdPerson/Blueprints/SpiderGameInstance.SpiderGameInstance_C|GetTastyFlies _output_get)
    (Development|SetHiddeninGame (Variables|Default|GetSphere) false true)
    (Collision|SetCollisionEnabled (Variables|Default|GetCollision) "QueryAndPhysics")))

(fn ConstructionScript)