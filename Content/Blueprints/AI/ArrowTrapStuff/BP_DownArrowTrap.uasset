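; Arrow trap that periodically fires volleys of arrows, active only when the game instance enables arrow traps.
; On BeginPlay it checks the player character type and SpiderGameInstance's ArrowTraps flag, then shows its mesh, enables collision and starts a looping FireArrow timer.
; Each FireArrow spawns a BP_Arrow at all six ArrowSpawn points, offsetting each point's pitch and yaw by a quarter turn to orient the arrows.
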(event Custom|FireArrow
  (bind _arrowspawn (Variables|Default|GetArrowSpawn))
  (bind _arrowspawn5 (Variables|Default|GetArrowSpawn5))
  (bind _arrowspawn1 (Variables|Default|GetArrowSpawn1))
  (bind _arrowspawn2 (Variables|Default|GetArrowSpawn2))
  (bind _arrowspawn3 (Variables|Default|GetArrowSpawn3))
  (bind _arrowspawn4 (Variables|Default|GetArrowSpawn4))
  (bind _returnvalue (Transformation|GetWorldRotation _arrowspawn5))
  (bind _returnvalue_2 (Transformation|GetWorldRotation _arrowspawn))
  (bind _returnvalue_3 (Transformation|GetWorldRotation _arrowspawn1))
  (bind _returnvalue_4 (Transformation|GetWorldRotation _arrowspawn2))
  (bind _returnvalue_5 (Transformation|GetWorldRotation _arrowspawn3))
  (bind _returnvalue_6 (Transformation|GetWorldRotation _arrowspawn4))
  (bind (_roll _pitch _yaw) (Math|Rotator|BreakRotator _returnvalue))
  (bind (_roll_2 _pitch_2 _yaw_2) (Math|Rotator|BreakRotator _returnvalue_2))
  (bind (_roll_3 _pitch_3 _yaw_3) (Math|Rotator|BreakRotator _returnvalue_3))
  (bind (_roll_4 _pitch_4 _yaw_4) (Math|Rotator|BreakRotator _returnvalue_4))
  (bind (_roll_5 _pitch_5 _yaw_5) (Math|Rotator|BreakRotator _returnvalue_5))
  (bind (_roll_6 _pitch_6 _yaw_6) (Math|Rotator|BreakRotator _returnvalue_6))
  (Game|SpawnActorfromClass "/Game/Blueprints/AI/ArrowTrapStuff/BP_Arrow.BP_Arrow_C" (Math|Transform|MakeTransform (Transformation|GetWorldLocation _arrowspawn) (Math|Rotator|MakeRotator _roll_2 (+ _pitch_2 9e+01) (- _yaw_2 9e+01)) "1.000000,1.000000,1.000000") "Undefined" "MultiplyWithRoot" 0 0)
  (Game|SpawnActorfromClass "/Game/Blueprints/AI/ArrowTrapStuff/BP_Arrow.BP_Arrow_C" (Math|Transform|MakeTransform (Transformation|GetWorldLocation _arrowspawn1) (Math|Rotator|MakeRotator _roll_3 (+ _pitch_3 9e+01) (- _yaw_3 9e+01)) "1.000000,1.000000,1.000000") "Undefined" "MultiplyWithRoot" 0 0)
  (Game|SpawnActorfromClass "/Game/Blueprints/AI/ArrowTrapStuff/BP_Arrow.BP_Arrow_C" (Math|Transform|MakeTransform (Transformation|GetWorldLocation _arrowspawn2) (Math|Rotator|MakeRotator _roll_4 (+ _pitch_4 9e+01) (- _yaw_4 9e+01)) "1.000000,1.000000,1.000000") "Undefined" "MultiplyWithRoot" 0 0)
  (Game|SpawnActorfromClass "/Game/Blueprints/AI/ArrowTrapStuff/BP_Arrow.BP_Arrow_C" (Math|Transform|MakeTransform (Transformation|GetWorldLocation _arrowspawn3) (Math|Rotator|MakeRotator _roll_5 (+ _pitch_5 9e+01) (- _yaw_5 9e+01)) "1.000000,1.000000,1.000000") "Undefined" "MultiplyWithRoot" 0 0)
  (Game|SpawnActorfromClass "/Game/Blueprints/AI/ArrowTrapStuff/BP_Arrow.BP_Arrow_C" (Math|Transform|MakeTransform (Transformation|GetWorldLocation _arrowspawn4) (Math|Rotator|MakeRotator _roll_6 (+ _pitch_6 9e+01) (- _yaw_6 9e+01)) "1.000000,1.000000,1.000000") "Undefined" "MultiplyWithRoot" 0 0)
  (Game|SpawnActorfromClass "/Game/Blueprints/AI/ArrowTrapStuff/BP_Arrow.BP_Arrow_C" (Math|Transform|MakeTransform (Transformation|GetWorldLocation _arrowspawn5) (Math|Rotator|MakeRotator _roll (+ _pitch 9e+01) (- _yaw 9e+01)) "1.000000,1.000000,1.000000") "Undefined" "MultiplyWithRoot" 0 0))

(event EventBeginPlay
  (bind _staticmesh (Variables|Default|GetStaticMesh))
  (Utilities|Casting|CastToBP_ThirdPersonCharacter (Game|GetPlayerCharacter 0))
  (bind _asspider_game_instance (Utilities|Casting|CastToSpiderGameInstance (Game|GetGameInstance)))
  (if (Variables|/Game/ThirdPerson/Blueprints/SpiderGameInstance.SpiderGameInstance_C|GetArrow%20Traps _asspider_game_instance)
    (Utilities|Time|SetTimerbyFunctionName 0 "FireArrow" 3.0 true)
    (Development|SetHiddeninGame _staticmesh false false)
    (Collision|SetCollisionEnabled _staticmesh "QueryAndPhysics")))

(fn ConstructionScript)