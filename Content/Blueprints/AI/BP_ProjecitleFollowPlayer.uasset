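; Homing projectile actor that follows the first player's pawn.
; Each Tick it interpolates its rotation toward the player, using ProjectileSpeed as the turn rate, then steps along its forward vector by HomingStrength.
; The step is not scaled by delta time, so travel speed depends on frame rate.
; Movement is unswept, and the file contains no hit or damage logic.
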(event EventTick
  (params (DeltaSeconds :type Float%20%28single-precision%29))
  (bind _returnvalue (Transformation|GetActorRotation))
  (Transformation|SetActorRotation (Math|Interpolation|RInterpTo _returnvalue (Math|Rotator|FindLookatRotation (Transformation|GetActorLocation) (.Location (Math|Transform|BreakTransform (Transformation|GetActorTransform (Game|Player|GetPlayerPawn 0))))) DeltaSeconds (Variables|Default|GetProjectile%20Speed)))
  (Transformation|SetActorRelativeLocation (+ (* (Math|Vector|GetForwardVector _returnvalue) (Variables|Default|GetHoming%20Strength)) (Transformation|GetActorLocation))))

(fn ConstructionScript)