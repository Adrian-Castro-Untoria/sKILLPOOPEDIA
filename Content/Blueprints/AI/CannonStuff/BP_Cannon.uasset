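; Player-tracking cannon that becomes visible, collidable and active only when the Canons flag (skill tree setup) is set in SpiderGameInstance.
; On BeginPlay that flag starts a looping timer that spawns BP_Cannonball from the CannonballSpawn point.
; Tick turns PropCannon toward the player, remapping look-at axes to suit the mesh.
; Overlap with the Colli volume sets PlayerInside, which pauses both aiming and firing while the player is inside.
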(event OnComponentBeginOverlap(colli)
  (params (OverlappedComponent :type Primitive%20Component%20Object%20Reference) (OtherActor :type Actor%20Object%20Reference) (OtherComp :type Primitive%20Component%20Object%20Reference) (OtherBodyIndex :type Integer) (bFromSweep :type Boolean) (SweepResult :type Hit%20Result%20Structure%20%28by%20ref%29))
  (Utilities|Casting|CastToBP_ThirdPersonCharacter OtherActor)
  (Variables|Default|SetbPlayerInside true))

(event OnComponentEndOverlap(colli)
  (params (OverlappedComponent :type Primitive%20Component%20Object%20Reference) (OtherActor :type Actor%20Object%20Reference) (OtherComp :type Primitive%20Component%20Object%20Reference) (OtherBodyIndex :type Integer))
  (Utilities|Casting|CastToBP_ThirdPersonCharacter OtherActor)
  (Variables|Default|SetbPlayerInside false))

(event Custom|FireCannon
  (bind _cannonballspawn (Variables|Default|GetCannonballSpawn))
  (bind _returnvalue (Transformation|GetWorldRotation _cannonballspawn))
  (bind (_roll _pitch _yaw) (Math|Rotator|BreakRotator _returnvalue))
  ;[0.15 0 0.03163 0.5] Spawn
  (if (not (Variables|Default|GetbPlayerInside))
    (Game|SpawnActorfromClass "/Game/Blueprints/AI/CannonStuff/BP_Cannonball.BP_Cannonball_C" (Math|Transform|MakeTransform (Transformation|GetWorldLocation _cannonballspawn) (Math|Rotator|MakeRotator (* (+ _pitch 5.0) -1.0) (* (+ _roll 5.0) -1.0) (+ _yaw 9e+01)) "1.000000,1.000000,1.000000") "Undefined" "MultiplyWithRoot" 0 0)))

(event EventTick
  (params (DeltaSeconds :type Float%20%28single-precision%29))
  (bind _returnvalue (Game|GetPlayerCharacter 0))
  (bind _prop_cannon (Variables|Default|GetProp_Cannon))
  (bind _returnvalue_2 (Transformation|GetActorLocation _returnvalue))
  (bind _returnvalue_3 (Transformation|GetWorldLocation _prop_cannon))
  (bind _returnvalue_4 (Math|Rotator|FindLookatRotation _returnvalue_3 _returnvalue_2))
  (bind (_roll _pitch _yaw) (Math|Rotator|BreakRotator _returnvalue_4))
  ;[0.15 0.08439 0.01548 0.5] Rotation Cannon
  (if (not (Variables|Default|GetbPlayerInside))
    (Transformation|SetWorldRotation (Variables|Default|GetProp_Cannon) (Math|Rotator|MakeRotator (* _pitch -1.0) (* _roll -1.0) (- _yaw 9e+01)) false false)))

(event EventBeginPlay
  ;[0.000155 0.15 0.02388 0.5] Setup Skilltree
  (Utilities|Casting|CastToBP_ThirdPersonCharacter (Game|GetPlayerCharacter 0))
  (bind _asspider_game_instance (Utilities|Casting|CastToSpiderGameInstance (Game|GetGameInstance)))
  (if (Variables|/Game/ThirdPerson/Blueprints/SpiderGameInstance.SpiderGameInstance_C|GetCanons _asspider_game_instance)
    (Utilities|Time|SetTimerbyFunctionName 0 "FireCannon" 3.0 true)
    (Development|SetHiddeninGame (Variables|Default|GetProp_Cannon) false false)
    (Collision|SetCollisionEnabled (Variables|Default|GetBox) "QueryAndPhysics")))

(fn ConstructionScript)