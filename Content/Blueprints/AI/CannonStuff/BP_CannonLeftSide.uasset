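; BP_CannonLeftSide is an AI cannon, apparently the left-side variant, that fires cannonballs on a repeating timer.
; Tick sets PropCannon's world rotation from only the roll of a look-at toward the player, offset 90 degrees, with zero pitch and yaw, so it does not actually track the player.
; A looping BeginPlay timer calls FireCannon, spawning BP_Cannonball at CannonballSpawn with a yaw offset.
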(event Custom|FireCannon
  (bind _cannonballspawn (Variables|Default|GetCannonballSpawn))
  (bind _returnvalue (Transformation|GetWorldRotation _cannonballspawn))
  (bind (_roll _pitch _yaw) (Math|Rotator|BreakRotator _returnvalue))
  (Game|SpawnActorfromClass "/Game/Blueprints/AI/CannonStuff/BP_Cannonball.BP_Cannonball_C" (Math|Transform|MakeTransform (Transformation|GetWorldLocation _cannonballspawn) (Math|Rotator|MakeRotator _roll _pitch (+ _yaw -9e+01)) "1.000000,1.000000,1.000000") "Undefined" "MultiplyWithRoot" 0 0))

(event EventTick
  (params (DeltaSeconds :type Float%20%28single-precision%29))
  (Transformation|SetWorldRotation (Variables|Default|GetProp_Cannon) (Math|Rotator|MakeRotator (+ (.Roll (Math|Rotator|BreakRotator (Math|Rotator|FindLookatRotation (Transformation|GetWorldLocation (Variables|Default|GetProp_Cannon)) (Transformation|GetActorLocation (Game|GetPlayerCharacter 0))))) 9e+01) 0.0 0.0) false false))

(event EventBeginPlay
  (Utilities|Time|SetTimerbyFunctionName 0 "FireCannon" 3.0 true))

(fn ConstructionScript)