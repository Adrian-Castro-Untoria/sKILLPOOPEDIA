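; Homing fireball actor that chases the player and damages them through an overlap sphere.
; BeginPlay reveals the sphere and enables its collision only if the game instance's HomingFireball flag is set.
; Tick always turns toward the player pawn and steps forward by HomingStrength, independent of frame time.
; While any Character overlaps the sphere, the player takes damage every tick.
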(event OnComponentBeginOverlap(Sphere)
  (params (OverlappedComponent :type Primitive%20Component%20Object%20Reference) (OtherActor :type Actor%20Object%20Reference) (OtherComp :type Primitive%20Component%20Object%20Reference) (OtherBodyIndex :type Integer) (bFromSweep :type Boolean) (SweepResult :type Hit%20Result%20Structure%20%28by%20ref%29))
  (Class|KismetSystemLibrary|IsObjectOfSoftClass OtherActor "/Script/Engine.Character"
    (:True
      (Variables|Default|SetIsTouchingBall true))))

(event OnComponentEndOverlap(Sphere)
  (params (OverlappedComponent :type Primitive%20Component%20Object%20Reference) (OtherActor :type Actor%20Object%20Reference) (OtherComp :type Primitive%20Component%20Object%20Reference) (OtherBodyIndex :type Integer))
  (Class|KismetSystemLibrary|IsObjectOfSoftClass OtherActor "/Script/Engine.Character"
    (:True
      (Variables|Default|SetIsTouchingBall false))))

(event EventBeginPlay
  (bind _sphere (Variables|Default|GetSphere))
  (bind _asspider_game_instance (Utilities|Casting|CastToSpiderGameInstance (Game|GetGameInstance)))
  (Variables|Ref|SetGameInstance_Ref _asspider_game_instance)
  (bind _asbp_third_person_character (Utilities|Casting|CastToBP_ThirdPersonCharacter (Game|GetPlayerCharacter 0)))
  (Variables|Ref|SetCharacter_Ref _asbp_third_person_character)
  (if (Variables|/Game/ThirdPerson/Blueprints/SpiderGameInstance.SpiderGameInstance_C|GetHomingFireball (Variables|Ref|GetGameInstance_Ref))
    (Development|SetHiddeninGame _sphere false false)
    (Collision|SetCollisionEnabled _sphere "QueryAndPhysics")))

(event EventTick
  (params (DeltaSeconds :type Float%20%28single-precision%29))
  (bind _returnvalue (Game|Player|GetPlayerPawn 0))
  (bind _returnvalue_2 (Transformation|GetActorRotation))
  (if true
    (Utilities|IsValid _returnvalue
      (:Is%20Valid
        (Transformation|SetActorRotation (Math|Interpolation|RInterpTo _returnvalue_2 (Math|Rotator|FindLookatRotation (Transformation|GetActorLocation) (.Location (Math|Transform|BreakTransform (Transformation|GetActorTransform _returnvalue)))) DeltaSeconds (Variables|Default|GetProjectile%20Speed)))
        (Transformation|SetActorRelativeLocation (+ (* (Math|Vector|GetForwardVector _returnvalue_2) (Variables|Default|GetHoming%20Strength)) (Transformation|GetActorLocation)))
        (if (Variables|Default|GetIsTouchingBall)
          (Default|TakingDamage (Variables|Ref|GetCharacter_Ref) (Variables|Default|GetDamageValue)))))))

(fn ConstructionScript)